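; BP_PlayerParent is a base player character Blueprint that creates the action menu widget and handles death and respawn.
; On death it disables movement, waits briefly, then moves the capsule to the current room's RESPAWN point.
; It then undoes the ragdoll by resetting and reattaching the mesh, restores movement and collision, resets an attribute from another, and marks the player alive.
; Pressing X triggers Die directly.
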(event Custom|Dead
  (bind _capsulecomponent (Variables|Default|GetCapsuleComponent))
  (bind _mesh (Variables|Character|GetMesh))
  (Pawn|Components|CharacterMovement|SetMovementMode (Variables|Character|GetCharacterMovement) "MOVE_None" 0)
  (Utilities|FlowControl|Delay 2.0)
  (Transformation|SetWorldLocation (Variables|Default|GetCapsuleComponent) (+ (Transformation|GetWorldLocation (Variables|/Game/_Project/cruey/Minigame_System/BP_Room.BP_Room_C|GetRESPAWN (.AsBP%20Room (CallFunction|GetCurrentRoom self)))) "0, 0,55.000000") false false)
  (Physics|SetSimulatePhysics _mesh false)
  (Class|SkeletalMeshComponent|ResetAllBodiesSimulatePhysics _mesh)
  (Transformation|ResetRelativeTransform _mesh)
  (Transformation|AttachComponentToComponent _mesh _capsulecomponent "None" "KeepWorld" "KeepWorld" "KeepWorld" true)
  (Transformation|SetRelativeLocation _mesh "0, 0,-90.000000" false false)
  (Transformation|SetRelativeRotation _mesh "0,-90.000000, 0" false false)
  (Pawn|Components|CharacterMovement|SetMovementMode (Variables|Character|GetCharacterMovement) "MOVE_Walking" 0)
  (Collision|SetCollisionResponsetoChannel _capsulecomponent "ECC_Pawn" "ECR_Block")
  (Collision|SetCollisionEnabled (Variables|Character|GetMesh) "QueryAndPhysics")
  (CallFunction|SetAttribute "NewEnumerator0" (CallFunction|GetAttribute "NewEnumerator1"))
  (Variables|Default|SetisAlive true))

(event EventBeginPlay)

(event Collision|EventActorBeginOverlap
  (params (OtherActor :type Actor%20Object%20Reference)))

(event EventBeginPlayPlayer
  (EventDispatchers|BindEventtoOnDeath (delegate Custom|Dead))
  (bind _returnvalue (UserInterface|CreateWidget "/Game/_Project/cruey/W_ActionMenu.W_ActionMenu_C" (Game|GetPlayerController 0)))
  (UserInterface|Viewport|AddtoViewport _returnvalue 0))

(event Input|KeyboardEvents|X
  (params (Key :type Key%20Structure :default "None"))
  (:Pressed
    (CallFunction|Die)))

(fn ConstructionScript
  (|CallParentFunction))
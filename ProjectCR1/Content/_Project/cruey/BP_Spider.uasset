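; Spider enemy that chases a player target and lunges at it, dealing damage or occasionally starting a hack minigame on hit.
; Tick drives the AI through lock timers: find target, AIMoveTo, then a montage notify starts the lunge.
; The leap interpolates the capsule along a forward line trace up to a distance limit, with animation frozen.
; Trace or collision hits can stun it, pausing its logic for a daze period.
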(event OnComponentHit(CapsuleComponent)
  (params (HitComponent :type Primitive%20Component%20Object%20Reference) (OtherActor :type Actor%20Object%20Reference) (OtherComp :type Primitive%20Component%20Object%20Reference) (NormalImpulse :type Vector :default "0, 0, 0") (Hit :type Hit%20Result%20Structure%20%28by%20ref%29))
  ;[1 1 1] Push the player on collision
  (if (Variables|Default|GetisLunging)
    (Utilities|FlowControl|Sequence
      (:then_0
        (Utilities|Casting|CastToBP_PlayerParent OtherActor)
        (Development|PrintString "xxwxw"))
      (:then_1
        (Variables|Default|SetisLunging false)
        (Variables|/Script/Engine.SkeletalMeshComponent|SetGlobalAnimRateScale (Variables|Character|GetMesh) 1.0)
        (CallFunction|Stunned))
      (:then_2
        (if (not (Variables|/Game/_Project/BP/Core/BP_GI.BP_GI_C|GetHackGameActive (CallFunction|GetGamexInstance self)))
          (if (> (Math|Random|RandomIntegerinRange 0 100) 15)
            (Game|Damage|ApplyDamage (stale _asbp_player_parent) (Math|Conversions|ToFloat(Integer) (CallFunction|GetAttribute "NewEnumerator2")) 0 0)
            (else
              (CallFunction|StartHackGame self))))))
    (else
      (bind _asbp_player_parent (Utilities|Casting|CastToBP_PlayerParent OtherActor)))))

(event OnComponentHit(Mesh)
  (params (HitComponent :type Primitive%20Component%20Object%20Reference) (OtherActor :type Actor%20Object%20Reference) (OtherComp :type Primitive%20Component%20Object%20Reference) (NormalImpulse :type Vector :default "0, 0, 0") (Hit :type Hit%20Result%20Structure%20%28by%20ref%29))
  (if (Variables|Default|GetisLunging)
    (Utilities|Casting|CastToBP_PlayerParent OtherActor
      (:then
        (Development|PrintString "xx"))
      (:CastFailed
        (Variables|Default|SetisLunging false)
        (Variables|/Script/Engine.SkeletalMeshComponent|SetGlobalAnimRateScale (Variables|Character|GetMesh) 1.0)
        (CallFunction|Stunned)))))

(event Custom|Stunned
  (Variables|Default|SetisDazed true)
  (Variables|/Script/Engine.SkeletalMeshComponent|SetGlobalAnimRateScale (Variables|Character|GetMesh) 1.0)
  (Utilities|FlowControl|Delay 0.2)
  (Animation|Montage|PlayMontage (Variables|Character|GetMesh) "/Game/Spiders/Animations/Spider2/A_death1_Montage.A_death1_Montage"
    (:OnNotifyBegin
      (Variables|/Script/Engine.SkeletalMeshComponent|SetGlobalAnimRateScale (Variables|Character|GetMesh) 0.0))))

(event EventBeginPlay
  (|CallParentFunction) ; This node is disabled and will not be called.\nDrag off pins to build functionality.
)

(event Collision|EventActorBeginOverlap
  (params (OtherActor :type Actor%20Object%20Reference))
  (|CallParentFunction OtherActor) ; This node is disabled and will not be called.\nDrag off pins to build functionality.
)

(event EventTick
  (params (DeltaSeconds :type Float%20%28single-precision%29))
  (bind _value (CallFunction|GetAttribute "NewEnumerator5"))
  (bind _capsulecomponent (Variables|Default|GetCapsuleComponent))
  (bind _p_ky_cutter1 (Variables|Default|GetP_ky_cutter1))
  (bind _returnvalue (Transformation|GetWorldLocation _capsulecomponent))
  (|CallParentFunction DeltaSeconds)
  (if (not (> (Variables|Default|GetFullLock_Time) 0.0))
    (if (Variables|Default|GetisDazed)
      (Rendering|SetVisibility _p_ky_cutter1 true false)
      (if (> (Variables|Default|GetDaze_Time) (Variables|Default|GetDaze_TimeMax))
        (Variables|Default|SetDaze_Time 0.0)
        (Variables|/Script/Engine.SkeletalMeshComponent|SetGlobalAnimRateScale (Variables|Character|GetMesh) 1.0)
        (Variables|Default|SetisDazed false)
        (else
          (Variables|Default|SetDaze_Time (+ (Variables|Default|GetDaze_Time) DeltaSeconds))))
      (else
        (Rendering|SetVisibility _p_ky_cutter1 false false)
        (Utilities|FlowControl|Sequence
          (:then_0
            (if (Variables|Default|GetisLunging)
              (bind _outhit (Collision|LineTraceByChannel _returnvalue (+ (* (Math|Vector|GetForwardVector _capsulecomponent) 125.0) _returnvalue) "TraceTypeQuery1" false 0 "ForOneFrame"))
              (if (.bBlockingHit (Collision|BreakHitResult _outhit))
                (Utilities|IsValid (.HitActor (Collision|BreakHitResult _outhit))
                  (:Is%20Valid
                    (bind _asbp_player_parent (Utilities|Casting|CastToBP_PlayerParent (.HitActor (Collision|BreakHitResult _outhit)))
                      (:then
                        ;[1 1 1] If Player hit = hack game triggered
                        (Variables|Default|SetisLunging false :!label _label)
                        (Variables|/Script/Engine.SkeletalMeshComponent|SetGlobalAnimRateScale (Variables|Character|GetMesh) 1.0)
                        (if (> (Math|Random|RandomIntegerinRange 0 100) 9)
                          (Game|Damage|ApplyDamage _asbp_player_parent (Math|Conversions|ToFloat(Integer) (CallFunction|GetAttribute "NewEnumerator2")) 0 0)
                          (else
                            (CallFunction|StartHackGame self))))
                      (:CastFailed
                        ;[1 1 1] If wall hit = stun
                        (Variables|Default|SetisLunging false)
                        (Variables|/Script/Engine.SkeletalMeshComponent|SetGlobalAnimRateScale (Variables|Character|GetMesh) 1.0)
                        (CallFunction|Stunned))))
                  (:Is%20Not%20Valid
                    (goto _label)))
                (Variables|Default|SetMax_LeapDistance_Current 0.0)
                (Variables|Default|SetLogicLockTime 2.0)
                (Transformation|SetWorldLocation (Variables|Default|GetCapsuleComponent) (Math|Interpolation|VInterpTo _returnvalue (Math|Vector|SelectVector (.ImpactPoint (Collision|BreakHitResult _outhit)) (.TraceEnd (Collision|BreakHitResult _outhit)) (.bBlockingHit (Collision|BreakHitResult _outhit))) (Utilities|Time|GetWorldDeltaSeconds) 18.0) false false :!label _label_2)
                (Animation|Montage|PlayMontage (Variables|Character|GetMesh) (Variables|Default|GetANIM_ATK1) 1.0 1.0)
                (elif (< (Variables|Default|GetMax_LeapDistance_Current) (Variables|Default|GetMax_LeapDistance))
                  (Variables|Default|SetMax_LeapDistance_Current (+ (Variables|Default|GetMax_LeapDistance_Current) (Math|Vector|VectorLength (- _returnvalue (Math|Interpolation|VInterpTo _returnvalue (Math|Vector|SelectVector (.ImpactPoint (Collision|BreakHitResult _outhit)) (.TraceEnd (Collision|BreakHitResult _outhit)) (.bBlockingHit (Collision|BreakHitResult _outhit))) (Utilities|Time|GetWorldDeltaSeconds) 18.0)))))
                  (goto _label_2)
                  (else
                    (Variables|Default|SetisLunging false)
                    (Variables|/Script/Engine.SkeletalMeshComponent|SetGlobalAnimRateScale (Variables|Character|GetMesh) 1.0)
                    (Variables|Default|SetMax_LeapDistance_Current 0.0))))))
          (:then_1
            (if (Variables|Default|GetisAlive)
              ;[1 1 1] is AI locked?
              (if (< (Variables|Default|GetLogicLockTime) 0.1)
                ;[1 1 1] has Target?
                (Utilities|IsValid (Variables|Default|GetTarget)
                  (:Is%20Valid
                    ;[1 1 1] Target Alive?
                    (if (Variables|/Game/_Project/cruey/BP_GameCharacter.BP_GameCharacter_C|GetisAlive (Variables|Default|GetTarget))
                      ;[1 1 1] in Range?
                      (if (< (Transformation|GetDistanceTo (Variables|Default|GetTarget) self) (Math|Conversions|ToFloat(Integer) _value))
                        (if (< (Transformation|GetDistanceTo (Variables|Default|GetTarget) self) (Math|Conversions|ToFloat(Integer) (/ _value 2)))
                          _
                          (else
                            _))
                        (if (not (Variables|Default|GetisLunging))
                          ;[1 1 1] Begin Lunge
                          (Variables|Default|SetLogicLockTime 2.0)
                          (Utilities|FlowControl|Delay 1.0)
                          (Components|Movement|StopMovementImmediately (Variables|Character|GetCharacterMovement))
                          (Animation|Montage|PlayMontage (Variables|Character|GetMesh) (Variables|Default|GetANIM_ATK1) 0.2
                            (:OnNotifyBegin
                              (Variables|Default|SetLungeStartLoc (Transformation|GetWorldLocation (Variables|/Script/Engine.Character|GetCapsuleComponent (Variables|Default|GetTarget))))
                              (Transformation|SetWorldRotation (Variables|Default|GetCapsuleComponent) (Math|Rotator|MakeRotator 0.0 0.0 (.yaw (Math|Rotator|FindLookatRotation (Transformation|GetWorldLocation (Variables|Default|GetCapsuleComponent)) (Transformation|GetWorldLocation (Variables|/Script/Engine.Character|GetCapsuleComponent (Variables|Default|GetTarget)))))) false false)
                              (Variables|Default|SetisLunging true)
                              (Variables|/Script/Engine.SkeletalMeshComponent|SetGlobalAnimRateScale (Variables|Character|GetMesh) 0.0))))
                        (else
                          ;[1 1 1] Move to
                          (if (not (Variables|Default|GetisLunging))
                            (AI|AIMoveTo self (Transformation|GetActorLocation (Variables|Default|GetTarget)) (Variables|Default|GetTarget) 66.0 false))))
                      (else
                        (Variables|Default|SetTarget 0))))
                  (:Is%20Not%20Valid
                    ;[1 1 1] Find Target
                    (CallFunction|FindTarget)
                    (Variables|Default|SetLogicLockTime 1.0)))
                (else
                  (Variables|Default|SetLogicLockTime (- (Variables|Default|GetLogicLockTime) DeltaSeconds)))))))))))

(fn ConstructionScript
  (|CallParentFunction))
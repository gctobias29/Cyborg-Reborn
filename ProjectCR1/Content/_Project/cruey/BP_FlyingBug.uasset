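; BP_FlyingBug is a ranged enemy AI that shoots projectiles at its target and nudges players it collides with.
; Tick runs the logic behind lock timers, finding a target, chasing when out of range or very close, and repositioning within half range, sidestepping when a box trace hits.
; Otherwise it plays an attack montage whose notify spawns BP_Projectile, cancelling if the target gets too close, and pauses after two shots.
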(event OnComponentHit(CapsuleComponent)
  (params (HitComponent :type Primitive%20Component%20Object%20Reference) (OtherActor :type Actor%20Object%20Reference) (OtherComp :type Primitive%20Component%20Object%20Reference) (NormalImpulse :type Vector :default "0, 0, 0") (Hit :type Hit%20Result%20Structure%20%28by%20ref%29))
  ;[1 1 1] Push the player on collision
  (bind _asbp_player_parent (Utilities|Casting|CastToBP_PlayerParent OtherActor))
  (Character|LaunchCharacter _asbp_player_parent (* (Math|Vector|GetForwardVector (Math|Rotator|FindLookatRotation (Transformation|GetWorldLocation (Variables|Default|GetCapsuleComponent)) (Transformation|GetWorldLocation (Variables|/Script/Engine.Actor|GetRootComponent _asbp_player_parent)))) 155.0) false false))

(event EventBeginPlay
  (|CallParentFunction) ; This node is disabled and will not be called.\nDrag off pins to build functionality.
)

(event Collision|EventActorBeginOverlap
  (params (OtherActor :type Actor%20Object%20Reference))
  (|CallParentFunction OtherActor) ; This node is disabled and will not be called.\nDrag off pins to build functionality.
)

(event EventTick
  (params (DeltaSeconds :type Float%20%28single-precision%29))
  (bind _returnvalue (Transformation|GetActorLocation))
  (bind _value (CallFunction|GetAttribute "NewEnumerator5"))
  (bind _value_2 (CallFunction|GetAttribute "NewEnumerator5"))
  (bind _self self)
  (bind _mesh (Variables|Character|GetMesh))
  (bind _anim_atk1 (Variables|Default|GetANIM_ATK1))
  (bind _capsulecomponent (Variables|Default|GetCapsuleComponent))
  (bind _returnvalue_2 (Math|Conversions|ToFloat(Integer) _value))
  (bind _returnvalue_3 (Math|Conversions|ToFloat(Integer) _value_2))
  (|CallParentFunction DeltaSeconds)
  (if (not (Variables|Default|GetIsBeingAttacked))
    (if (and (< (Variables|Default|GetFullLock_Time) 0.1) (Variables|Default|GetisAlive))
      ;[1 1 1] is AI locked?
      (if (< (Variables|Default|GetLogicLockTime) 0.1)
        ;[1 1 1] has Target?
        (Utilities|IsValid (Variables|Default|GetTarget)
          (:Is%20Valid
            ;[1 1 1] Target Alive?
            (if (Variables|/Game/_Project/cruey/BP_GameCharacter.BP_GameCharacter_C|GetisAlive (Variables|Default|GetTarget))
              ;[1 1 1] in Range?
              (if (< (Transformation|GetDistanceTo (Variables|Default|GetTarget) self) _returnvalue_3)
                (if (< (Transformation|GetDistanceTo (Variables|Default|GetTarget) self) 6e+01)
                  ;[1 1 1] Move to
                  (AI|AIMoveTo self (Transformation|GetActorLocation (Variables|Default|GetTarget)) (Variables|Default|GetTarget) (- _returnvalue_3 1.2e+02) true :!label _label)
                  (elif (< (Transformation|GetDistanceTo (Variables|Default|GetTarget) self) (Math|Conversions|ToFloat(Integer) (/ _value_2 2)))
                    ;[1 1 1] Find Target within AttackRange & move to it
                    (Variables|Default|SetLogicLockTime 0.4)
                    (bind _returnvalue_4 (Class|KismetSystemLibrary|BoxTraceMulti _returnvalue (+ (* (Math|Vector|GetForwardVector (Class|KismetMathLibrary|NegateRotator (Math|Rotator|FindLookatRotation (Transformation|GetActorLocation (Variables|Default|GetTarget)) _returnvalue))) _returnvalue_2) _returnvalue) "50.000000,50.000000,50.000000" "0, 0, 0" "TraceTypeQuery1" false 0 "None" true :!label _label_2))
                    (if _returnvalue_4
                      (AI|AIMoveTo _self (+ (* (Math|Vector|GetRightVector (Class|KismetMathLibrary|NegateRotator (Math|Rotator|FindLookatRotation (Transformation|GetActorLocation (Variables|Default|GetTarget)) _returnvalue))) _returnvalue_2) _returnvalue) 0 48.0 false
                        (:OnFail
                          (goto _label_2)))
                      (else
                        (AI|AIMoveTo _self (+ (* (Math|Vector|GetForwardVector (Class|KismetMathLibrary|NegateRotator (Math|Rotator|FindLookatRotation (Transformation|GetActorLocation (Variables|Default|GetTarget)) _returnvalue))) _returnvalue_2) _returnvalue) 0 48.0 false
                          (:OnFail
                            (goto _label_2)))))
                    (elif (>= (Variables|Default|GetShootTimes) 2.0)
                      (Variables|Default|SetShootTimes 0.0)
                      (Variables|Default|SetLogicLockTime 3.0)
                      (Variables|Default|SetMaxShootTimes (Math|Random|RandomIntegerinRange 1 3))
                      (else
                        (Math|Float|IncrementFloat (Variables|Default|GetShootTimes)
                          (:%20%20
                            ;[1 0.1419 0.2202] Attack: Shoot a fireball towards the player
                            (Animation|Montage|PlayMontage _mesh _anim_atk1
                              (:then
                                (bind _returnvalue_5 (Animation|GetPlayLength _anim_atk1))
                                (Variables|Default|SetLogicLockTime _returnvalue_5))
                              (:OnNotifyBegin
                                (if (< (Transformation|GetDistanceTo (Variables|Default|GetTarget) self) (Math|Conversions|ToFloat(Integer) (/ _value_2 2)))
                                  (Audio|Components|Audio|Stop _mesh)
                                  (else
                                    (CallFunction|RotatetoFaceTarget (Variables|Default|GetTarget))
                                    (Game|SpawnActorfromClass "/Game/_Project/cruey/BP_Projectile.BP_Projectile_C" (Math|Transform|MakeTransform (+ (Transformation|GetWorldLocation _capsulecomponent) (* (Math|Vector|GetForwardVector _capsulecomponent) 35.0) "0,0,45.000000") (Math|Rotator|MakeRotator 0.0 0.0 (.yaw (Transformation|GetWorldRotation (Variables|Default|GetCapsuleComponent)))) "1,1,1") "Undefined" self 0)))))))))))
                (else
                  (goto _label)))
              (else
                (Variables|Default|SetTarget 0))))
          (:Is%20Not%20Valid
            ;[1 1 1] Find Target
            (CallFunction|FindTarget)
            (Variables|Default|SetLogicLockTime 1.0)))
        (else
          (Variables|Default|SetLogicLockTime (- (Variables|Default|GetLogicLockTime) DeltaSeconds)))))))

(fn ConstructionScript
  (|CallParentFunction))
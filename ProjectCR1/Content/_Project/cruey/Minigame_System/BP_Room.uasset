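; BP_Room is one link in an endless chain of minigame combat rooms, each leading to the next once its monsters are dead.
; Once started and four seconds old, Tick prunes dead monsters and calls LevelUp when none remain.
; LevelUp runs once, raising MinigameLevel and placing a random room at NEXT.
; It fills that room's billboard points with level-scaled monsters, using a re-created seeded stream that repeats one type, then starts it.
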(event Custom|LevelUp
  (bind _self self)
  (bind _self_2 self)
  (bind _self_3 self)
  (bind _minigame_roomtypes (CallFunction|GetRoomTypes _self))
  (bind _minigame_monstertypes (CallFunction|GetMonsterTypes _self_2))
  (bind _asbp_gi (CallFunction|GetGamexInstance _self_3))
  (if (not (Variables|Default|GetRoomComplete))
    (Variables|/Game/_Project/BP/Core/BP_GI.BP_GI_C|SetMinigame_Level _asbp_gi (+ (Variables|/Game/_Project/BP/Core/BP_GI.BP_GI_C|GetMinigame_Level _asbp_gi) 1))
    (Variables|Default|SetRoomComplete true)
    (bind _returnvalue (Game|SpawnActorfromClass (Utilities|Array|Get(acopy) _minigame_roomtypes (Math|Random|RandomIntegerinRange 0 (- (Utilities|Array|Length _minigame_roomtypes) 1))) (Math|Transform|MakeTransform "0, 0, 0" "0, 0, 0" "1,1,1") "AlwaysSpawn" 0 0))
    (Transformation|SetWorldScale3D (Variables|BP_Room_C|GetSTART _returnvalue) "5.000000,5.000000,1.000000")
    (Transformation|SetWorldLocation (Variables|BP_Room_C|GetSTART _returnvalue) (Transformation|GetWorldLocation (Variables|Default|GetNEXT)) false false)
    (Utilities|FlowControl|Delay 2.0)
    (for _index (range 0 (- (Class|SceneComponent|GetNumChildrenComponents (Variables|BP_Room_C|GetBillboard _returnvalue)) 1))
      (bind _returnvalue_2 (Game|SpawnActorfromClass (Utilities|Array|Get(acopy) _minigame_monstertypes (Math|Random|RandomIntegerinRangefromStream 0 (- (Utilities|Array|Length _minigame_monstertypes) 1) (Math|Random|MakeRandomStream (Variables|Default|Getrng)))) (Math|Transform|MakeTransform (+ (Transformation|GetWorldLocation (Components|GetChildComponent (Variables|BP_Room_C|GetBillboard _returnvalue) _index)) "0, 0,125.000000") "0, 0, 0" "1,1,1") "Undefined" 0 0))
      (Utilities|IsValid _returnvalue_2
        (:Is%20Valid
          (Default|SetAttribute _returnvalue_2 "NewEnumerator0" (* (Default|GetAttribute _returnvalue_2 "NewEnumerator1") (Variables|/Game/_Project/BP/Core/BP_GI.BP_GI_C|GetMinigame_Level (CallFunction|GetGamexInstance self))))
          (Default|SetAttribute _returnvalue_2 "NewEnumerator1" (* (Default|GetAttribute _returnvalue_2 "NewEnumerator1") (Variables|/Game/_Project/BP/Core/BP_GI.BP_GI_C|GetMinigame_Level (CallFunction|GetGamexInstance self))))
          (Default|SetAttribute _returnvalue_2 "NewEnumerator2" (* (Default|GetAttribute _returnvalue_2 "NewEnumerator2") (Variables|/Game/_Project/BP/Core/BP_GI.BP_GI_C|GetMinigame_Level (CallFunction|GetGamexInstance self))))
          (Utilities|Array|Add (Variables|BP_Room_C|GetMonsters _returnvalue) _returnvalue_2)
          (bind _asbillboard_component (Utilities|Casting|CastToBillboardComponent (Components|GetChildComponent (Variables|BP_Room_C|GetBillboard _returnvalue) _index)))
          (Development|SetHiddeninGame (Components|GetChildComponent (Variables|BP_Room_C|GetBillboard _returnvalue) _index) true false))))
    (Variables|BP_Room_C|SetRoomStarted _returnvalue true)
    (bind _outactors (Actor|GetAllActorsOfClass "/Script/NavigationSystem.NavMeshBoundsVolume"))))

(event EventBeginPlay
  (Variables|Default|Setrng (Math|Random|RandomInteger 255)))

(event Collision|EventActorBeginOverlap
  (params (OtherActor :type Actor%20Object%20Reference)))

(event EventTick
  (params (DeltaSeconds :type Float%20%28single-precision%29))
  (bind _monsters (Variables|Default|GetMonsters))
  (if (Variables|Default|GetRoomStarted)
    (if (> (Actor|GetGameTimeSinceCreation) 4.0)
      (Utilities|FlowControl|Sequence
        (:then_0
          (if (== (Utilities|Array|Length _monsters) 0)
            (CallFunction|LevelUp)))
        (:then_1
          (for (_array_element _array_index) _monsters
            (if (Math|Boolean|Equal(Boolean) (Variables|/Game/_Project/cruey/BP_GameCharacter.BP_GameCharacter_C|GetisAlive _array_element) false)
              (Utilities|Array|RemoveIndex _monsters _array_index))))))))

(fn ConstructionScript)
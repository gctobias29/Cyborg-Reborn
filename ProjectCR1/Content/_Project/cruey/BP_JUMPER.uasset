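; BP_JUMPER is a monster enemy that chases a target and alternates between jump-slam and spin-dash attacks every 20 seconds.
; Monster2Tick drives both as flag-based state machines with VInterpTo movement, paced by LogicLockTime.
; The jump shows a decal, rises, relocates above the target, then slams, box-tracing to damage and launch players.
; The spin telegraphs with a static mesh, then dashes through pawns toward the Box component's location, randomly dealing reduced damage.
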(event Custom|Jumper_ondeath
  (Components|DestroyComponent (Variables|Default|GetDecal)))

(event EventBeginPlay
  (|CallParentFunction)
  (EventDispatchers|BindEventtoOnDeath (delegate Custom|Jumper_ondeath)))

(event Collision|EventActorBeginOverlap
  (params (OtherActor :type Actor%20Object%20Reference))
  (|CallParentFunction OtherActor) ; This node is disabled and will not be called.\nDrag off pins to build functionality.
)

(event EventMonster2Tick
  (bind _value (CallFunction|GetAttribute "NewEnumerator5"))
  (bind _capsulecomponent (Variables|Default|GetCapsuleComponent))
  (bind _target (Variables|Default|GetTarget))
  (bind _staticmesh (Variables|Default|GetStaticMesh))
  (bind _capsulecomponent_2 (Variables|Default|GetCapsuleComponent))
  (bind _mesh (Variables|Character|GetMesh))
  (bind _mesh_2 (Variables|Character|GetMesh))
  (bind _target_2 (Variables|Default|GetTarget))
  (bind _capsulecomponent_3 (Variables|Default|GetCapsuleComponent))
  (bind _capsulecomponent_4 (Variables|Default|GetCapsuleComponent))
  (bind _capsulecomponent_5 (Variables|Default|GetCapsuleComponent))
  (bind _capsulecomponent_6 (Variables|Default|GetCapsuleComponent))
  (bind _returnvalue (Transformation|GetWorldLocation _capsulecomponent_6))
  (bind _returnvalue_2 (Transformation|GetWorldLocation _capsulecomponent))
  (bind _returnvalue_3 (Transformation|GetWorldLocation _capsulecomponent_2))
  (bind _returnvalue_4 (Transformation|GetWorldLocation _capsulecomponent_4))
  (bind _capsulecomponent_7 (Variables|/Script/Engine.Character|GetCapsuleComponent _target))
  (bind _returnvalue_5 (Transformation|GetWorldLocation _capsulecomponent_7))
  (if (not (> (Variables|Default|GetFullLock_Time) 0.0))
    (Utilities|FlowControl|Sequence
      (:then_0
        (bind _output_get (Variables|Default|SetDelta%20Seconds_0 (Utilities|Time|GetWorldDeltaSeconds)))
        (if (Variables|Default|GetisAlive)
          (|SwitchSkill
            (:then_0
              (if (> (Variables|Default|GetLogicLockTime) 0.0)
                (Variables|Default|SetLogicLockTime (- (Variables|Default|GetLogicLockTime) _output_get))
                (else
                  (Utilities|IsValid _target_2
                    (:Is%20Valid
                      (if (Variables|Default|GetuseJumpAttack)
                        (if (Variables|Default|GetJumpAttack_Started)
                          (if (Math|Vector|Equal(Vector) _returnvalue_2 (Variables|Default|GetTargetLoc) 111.0)
                            (if (Variables|Default|GetJumpAttack_Relocated)
                              (if (Math|Vector|Equal(Vector) (Transformation|GetWorldLocation (Variables|Default|GetCapsuleComponent)) (Variables|Default|GetTargetLoc) 111.0)
                                (if (Variables|Default|GetJumpAttack_LandedStarted)
                                  (if (Math|Vector|Equal(Vector) (Transformation|GetWorldLocation (Variables|Default|GetCapsuleComponent)) (Variables|Default|GetTargetLoc) 222.0)
                                    (bind _outhits (Class|KismetSystemLibrary|BoxTraceMulti _returnvalue _returnvalue "200.000000,200.000000,500.000000" "0, 0, 0" "TraceTypeQuery1" false 0 "None" true))
                                    (for _array_element _outhits
                                      (bind _asbp_player_character (Utilities|Casting|CastToBP_PlayerCharacter (.HitActor (Collision|BreakHitResult _array_element))))
                                      (Character|LaunchCharacter _asbp_player_character (+ (* (Math|Vector|GetForwardVector (Math|Rotator|FindLookatRotation (Transformation|GetWorldLocation (Variables|Default|GetCapsuleComponent)) (Transformation|GetWorldLocation (Variables|/Script/Engine.Character|GetMesh _asbp_player_character)))) 5555.0) "0, 0,155.000000") true true)
                                      (Game|Damage|ApplyDamage _asbp_player_character (Math|Conversions|ToFloat(Integer) (CallFunction|GetAttribute "NewEnumerator2")) 0 0)
                                      (Effects|SpawnEmitteratLocation "/Game/AdvancedMagicFX13/Particles/P_ky_impact.P_ky_impact" (.ImpactPoint (Collision|BreakHitResult _array_element)) "0, 0, 0" (Transformation|GetWorldScale (Variables|Character|GetMesh))))
                                    (Variables|Default|SetJumpAttack_Started false)
                                    (Variables|Default|SetJumpAttack_Relocated false)
                                    (Variables|Default|SetJumpAttack_LandedStarted false)
                                    (Variables|Default|SetJumpAttack_ false)
                                    (Pawn|Components|CharacterMovement|SetMovementMode (Variables|Character|GetCharacterMovement) "MOVE_Walking" 0)
                                    (Variables|Default|SetLogicLockTime 3.0)
                                    (Components|Animation|SetAnimationMode (Variables|Character|GetMesh) "AnimationBlueprint")
                                    (else
                                      (Transformation|SetWorldLocation (Variables|Default|GetCapsuleComponent) (Math|Interpolation|VInterpTo (Transformation|GetWorldLocation (Variables|/Script/Engine.Character|GetCapsuleComponent (Variables|Default|GetTarget))) (Variables|Default|GetTargetLoc) (Variables|Default|GetDelta%20Seconds_0) 1.0) false false)))
                                  (else
                                    (Variables|Default|SetTargetLoc (- (stale _output_get_2) "0, 0,333.000000"))
                                    (Variables|Default|SetJumpAttack_LandedStarted true)
                                    (Components|Animation|PlayAnimation (Variables|Character|GetMesh) "/Game/SFB_DevilsPack/Animations/Devil_Attack3_Anim.Devil_Attack3_Anim" false)))
                                (else
                                  (Transformation|SetWorldLocation (Variables|Default|GetCapsuleComponent) (Math|Interpolation|VInterpTo _returnvalue_5 (Variables|Default|GetTargetLoc) (Variables|Default|GetDelta%20Seconds_0) 1.0) false false)))
                              (else
                                (Variables|Default|SetJumpAttack_Relocated true)
                                (bind _output_get_2 (Variables|Default|SetTargetLoc (+ _returnvalue_5 "0, 0,333.000000")))))
                            (else
                              (Transformation|SetWorldLocation (Variables|Default|GetCapsuleComponent) (Math|Interpolation|VInterpTo _returnvalue_2 (Variables|Default|GetTargetLoc) (Variables|Default|GetDelta%20Seconds_0) (Math|Float|SelectFloat 2.0 0.0 (Variables|Default|GetJumpAttack_Relocated))) false false)))
                          (else
                            (Variables|Default|SetJumpAttack_Started true)
                            (Variables|Default|SetTargetLoc (+ (* (Math|Vector|GetUpVector _capsulecomponent) 333.0) _returnvalue_2))
                            (Pawn|Components|CharacterMovement|SetMovementMode (Variables|Character|GetCharacterMovement) "MOVE_None" 0)
                            (Components|Animation|PlayAnimation (Variables|Character|GetMesh) "/Game/SFB_DevilsPack/Animations/Mannequin_Retarget/ThirdPersonJump_Start.ThirdPersonJump_Start" false)))
                        (else
                          (Utilities|FlowControl|Sequence
                            (:then_0
                              (Utilities|FlowControl|Sequence
                                (:then_1
                                  (if (Variables|Default|GetSpinStarted)
                                    (if (Variables|Default|GetisSpinning)
                                      (if (Math|Vector|Equal(Vector) (Variables|Default|GetSpinDestination) _returnvalue_4 156.0)
                                        (Collision|SetCollisionResponsetoChannel _capsulecomponent_3 "ECC_Pawn" "ECR_Block")
                                        (Variables|Default|SetisSpinning false)
                                        (Variables|Default|SetSpinStarted false)
                                        (Variables|Default|SetLogicLockTime 1.5)
                                        (Variables|/Script/Engine.SkeletalMeshComponent|SetGlobalAnimRateScale _mesh_2 1.0)
                                        (Components|Animation|SetAnimationMode _mesh_2 "AnimationBlueprint")
                                        (else
                                          (Collision|SetCollisionResponsetoChannel _capsulecomponent_3 "ECC_Pawn" "ECR_Ignore")
                                          (Transformation|SetWorldLocation _capsulecomponent_4 (Math|Interpolation|VInterpTo _returnvalue_4 (Variables|Default|GetSpinDestination) (Variables|Default|GetDelta%20Seconds_0) 1.0) false false)
                                          (Transformation|AddLocalRotation _capsulecomponent_4 "0, 0, 0" false false)
                                          (if (< (Math|Random|RandomIntegerinRange 0 1000) 100)
                                            (bind _outhit (Class|KismetSystemLibrary|BoxTraceSingleforObjects _returnvalue_3 _returnvalue_3 "155.000000,155.000000,255.000000" "0, 0, 0" (Utilities|Array|MakeArray "ObjectTypeQuery3") false 0 "None" true))
                                            (Game|Damage|ApplyDamage (.HitActor (Collision|BreakHitResult _outhit)) (* (Math|Conversions|ToFloat(Integer) (CallFunction|GetAttribute "NewEnumerator2")) 0.3) 0 0)
                                            (Effects|SpawnEmitteratLocation "/Game/AdvancedMagicFX13/Particles/P_ky_impact.P_ky_impact" (.ImpactPoint (Collision|BreakHitResult _outhit)) "0, 0, 0" (* (Transformation|GetWorldScale (Variables|Character|GetMesh)) 0.3)))))
                                      (else
                                        (Development|SetHiddeninGame _staticmesh true false)
                                        (bind (_outhit_2 _returnvalue_6) (Collision|LineTraceByChannel (Transformation|GetWorldLocation _capsulecomponent_5) (Transformation|GetWorldLocation (Variables|Default|GetBox)) "TraceTypeQuery1" false 0 "None"))
                                        (Variables|Default|SetSpinDestination (.TraceEnd (Collision|BreakHitResult _outhit_2)))
                                        (Variables|Default|SetisSpinning true)
                                        (Components|Animation|PlayAnimation _mesh "/Game/SFB_DevilsPack/Animations/Devil_Attack4_Anim.Devil_Attack4_Anim" true)
                                        (Variables|/Script/Engine.SkeletalMeshComponent|SetGlobalAnimRateScale _mesh 2.0)))))))
                            (:then_1
                              (if (> _value (Math|Float|Truncate (Transformation|GetDistanceTo _target_2 self)))
                                (if (not (Variables|Default|GetSpinStarted))
                                  (Utilities|FlowControl|Sequence
                                    (:then_0
                                      (Transformation|SetWorldRotation _capsulecomponent_5 (Math|Rotator|MakeRotator 0.0 0.0 (.yaw (Math|Rotator|FindLookatRotation (Transformation|GetWorldLocation (Variables|Default|GetCapsuleComponent)) (Transformation|GetWorldLocation (Variables|/Script/Engine.Character|GetMesh (Variables|Default|GetTarget)))))) false false)
                                      (Development|SetHiddeninGame _staticmesh false false)
                                      (Variables|Default|SetLogicLockTime 1.0))
                                    (:then_1
                                      (Variables|Default|SetSpinStarted true))))
                                (elif (not (Variables|Default|GetisSpinning))
                                  (AI|AIMoveTo self "0, 0, 0" _target_2 (/ (Math|Conversions|ToFloat(Integer) _value) 2.0) false))))))))
                    (:Is%20Not%20Valid
                      (CallFunction|FindTarget)))))))
          (else
            (Development|SetHiddeninGame (Variables|Default|GetStaticMesh) true false))))
      (:then_1
        (Rendering|SetVisibility (Variables|Default|GetDecal) (select (Variables|Default|GetJumpAttack_Started) true false) false)))))

(fn ConstructionScript
  (|CallParentFunction)
  (Class|SkinnedMeshComponent|SetMasterPoseComponent (Variables|Default|GetSlotFive) (Variables|Character|GetMesh) true))
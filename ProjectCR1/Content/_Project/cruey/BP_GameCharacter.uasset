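; Base character for player and monsters, providing attributes, damage, death and HP widgets, with empty begin-play, tick and finisher hooks.
; Outside the hacking game, damage lowers the attribute, turns toward the attacker, shows numbers, plays a hit montage and briefly stuns monsters.
; Death ragdolls the mesh and decrements the player's engaged-enemy count.
; SendDamage can freeze monsters; F box-traces for a living monster under 20% health to trigger Finisher_1.
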(event Custom|SendDamage
  (params (DamagedActor :type Actor%20Object%20Reference) (BaseDamage :type Float%20%28single-precision%29) (DamageTypeClass :type Damage%20Type%20Class%20Reference) (Condition :type Boolean))
  (Variables|Default|SetLastDamagedActor DamagedActor)
  (Game|Damage|ApplyDamage DamagedActor BaseDamage 0 self DamageTypeClass)
  (bind _asbp_monster_parent (Utilities|Casting|CastToBP_MonsterParent DamagedActor))
  (CallFunction|DisableAIonHit _asbp_monster_parent)
  (Variables|/Game/_Project/cruey/BP_MonsterParent.BP_MonsterParent_C|Set_IsFrozen _asbp_monster_parent Condition)
  (if Condition
    (Development|PrintString "FROZEN")
    (Components|Movement|StopMovementImmediately (Variables|/Script/Engine.Character|GetCharacterMovement _asbp_monster_parent))
    (Pawn|Components|CharacterMovement|SetMovementMode (Variables|/Script/Engine.Character|GetCharacterMovement _asbp_monster_parent) "MOVE_None" 0)))

(event Custom|Die
  (params (Target :type Object%20Object%20Reference))
  (Default|CallOnDeath)
  (Variables|Default|SetisAlive false)
  (CallFunction|SetAttribute "NewEnumerator0")
  (Physics|SetSimulatePhysics (Variables|Character|GetMesh) true)
  (Collision|SetCollisionResponsetoChannel (Variables|Collision|GetCapsuleComponent) "ECC_Pawn" "ECR_Ignore")
  (Collision|SetCollisionEnabled (Variables|Character|GetMesh) "PhysicsOnly")
  (bind _asbp_player_character (Utilities|Casting|CastToBP_PlayerCharacter Target))
  (bind _result (Math|Integer|DecrementInt (Variables|/Game/_Project/BP/Player/BP_PlayerCharacter.BP_PlayerCharacter_C|GetCurrentEnemiesEngaged_0 _asbp_player_character))
    (:%20%20
      (bind _output_get (Variables|/Game/_Project/BP/Player/BP_PlayerCharacter.BP_PlayerCharacter_C|SetCurrentEnemiesEngaged_0 _asbp_player_character _result))
      (Development|PrintString (Utilities|String|BuildString(Integer) "" "Enemies Engaged : " _output_get)))))

(event Custom|CyborgTick
  (params (NewParam :type Float%20%28single-precision%29)))

(event Custom|BeginPlay_Monster)

(event Custom|Finisher_1
  (params (Target :type BP%20Monster%20Parent%20Object%20Reference)))

(event Custom|BeginPlay_Player)

(event Custom|MonsterTick)

(event Custom|Monster2Tick)

(event Custom|DisableAI_OnHit
  (bind _charactermovement (Variables|Character|GetCharacterMovement))
  (bind _asbp_monster_parent (Utilities|Casting|CastToBP_MonsterParent self))
  (Pawn|Components|CharacterMovement|SetMovementMode _charactermovement "MOVE_None" 0)
  (Variables|/Game/_Project/cruey/BP_MonsterParent.BP_MonsterParent_C|SetIsBeingAttacked _asbp_monster_parent true)
  (Utilities|FlowControl|RetriggerableDelay 0.33)
  (Pawn|Components|CharacterMovement|SetMovementMode _charactermovement "MOVE_Walking" 0)
  (Variables|/Game/_Project/cruey/BP_MonsterParent.BP_MonsterParent_C|SetIsBeingAttacked _asbp_monster_parent false))

(event EventBeginPlay
  (EventDispatchers|BindEventtoOnDamaged (delegate Custom|DisableAI_OnHit))
  (CallFunction|BeginPlayPlayer)
  (CallFunction|BeginPlayMonster)
  (bind _returnvalue (UserInterface|CreateWidget "/Game/_Project/cruey/W_HPBar.W_HPBar_C" 0 self))
  (UserInterface|SetWidget (Variables|Default|GetHP_Widget) _returnvalue)
  (bind _returnvalue_2 (UserInterface|CreateWidget "/Game/_Project/cruey/W_isDead.W_isDead_C" 0 self))
  (UserInterface|SetWidget (Variables|Default|GetDeathWidget) _returnvalue_2))

(event Collision|EventActorBeginOverlap
  (params (OtherActor :type Actor%20Object%20Reference)))

(event EventTick
  (params (DeltaSeconds :type Float%20%28single-precision%29))
  (Variables|Default|SetDelta%20Seconds DeltaSeconds)
  (CallFunction|CyborgTick DeltaSeconds)
  (CallFunction|MonsterTick)
  (CallFunction|Monster2Tick))

(event Game|Damage|EventAnyDamage
  (params (Damage :type Float%20%28single-precision%29) (DamageType :type Damage%20Type%20Object%20Reference) (InstigatedBy :type Controller%20Object%20Reference) (DamageCauser :type Actor%20Object%20Reference))
  (bind _value (CallFunction|GetAttribute "NewEnumerator0"))
  (bind _returnvalue (Math|Float|Truncate Damage))
  (bind _mesh (Variables|Character|GetMesh))
  (bind _anim_onhit (Variables|Default|GetANIM_ONHIT))
  (bind _returnvalue_2 (- _value _returnvalue))
  (bind _returnvalue_3 (Components|SkeletalMesh|GetAnimInstance _mesh))
  (if (not (Variables|/Game/_Project/BP/Core/BP_GI.BP_GI_C|GetHackGameActive (CallFunction|GetGamexInstance self)))
    (Default|CallOnDamaged)
    (if (< _returnvalue_2 1)
      (CallFunction|Die DamageCauser)
      (else
        (Default|CallOnDamaged)
        (CallFunction|SetAttribute "NewEnumerator0" _returnvalue_2)))
    (CallFunction|RotatetoFaceTarget DamageCauser)
    ;[1 1 1] create damage numbers widget
    (bind _returnvalue_4 (UserInterface|CreateWidget "/Game/_Project/cruey/W_Damage.W_Damage_C" 0 (Utilities|Text|ToText(Float) Damage "HalfToEven")))
    (bind _returnvalue_5 (AddComponent|AddWidgetComponent false))
    (UserInterface|SetWidget _returnvalue_5 _returnvalue_4)
    ;[1 1 1] if were not playing an animation, play OnHitAnim
    (Utilities|IsValid _returnvalue_3
      (:Is%20Valid
        (if (Class|AnimInstance|IsAnyMontagePlaying _returnvalue_3)
          (if (Animation|Montage|MontageIsPlaying _returnvalue_3 _anim_onhit)
            (Animation|Montage|PlayMontage _mesh _anim_onhit :!label _label))
          (else
            (goto _label)))))))

(event Input|KeyboardEvents|F
  (params (Key :type Key%20Structure :default "None"))
  (:Pressed
    (CallFunction|CheckFinisherTargets)))

(fn ConstructionScript)

(fn SetAttribute
  (params (AttributeType :type E_AttributeType%20Enum :default "NewEnumerator0") (Value :type Integer))
  (bind _attributes (Variables|Default|GetAttributes))
  (for (_array_element _array_index) _attributes
    (if (Utilities|Enum|Equal(Enum) (.AttributeType (Utilities|Struct|BreakS_AttributeType _array_element)) AttributeType)
      (bind _structout (Utilities|Struct|SetmembersinS_AttributeType _array_element Value))
      (Utilities|Array|SetArrayElem _attributes _array_index _structout))))

(fn GetAttribute
  (params (AttributeType :type E_AttributeType%20Enum :default "NewEnumerator0"))
  (for _array_element (Variables|Default|GetAttributes)
    (if (Utilities|Enum|Equal(Enum) (.AttributeType (Utilities|Struct|BreakS_AttributeType _array_element)) AttributeType)
      (return (.Value (Utilities|Struct|BreakS_AttributeType _array_element))))))

(fn GetTargetsfromTraceHits
  (params (Hit%20Results :type Array%20of%20Hit%20Result%20Structures))
  (bind _targets (LocalVariables|GetTargets))
  (for _array_element Hit%20Results
    (bind _asbp_game_character (Utilities|Casting|CastToBP_GameCharacter (.HitActor (Collision|BreakHitResult _array_element))))
    (if (Variables|BP_GameCharacter_C|GetisAlive _asbp_game_character)
      (if (Utilities|Array|ContainsItem (Variables|Default|GetTargetTypes) (Variables|BP_GameCharacter_C|GetTargetGroup _asbp_game_character))
        (if (not (Utilities|Array|ContainsItem _targets _asbp_game_character))
          (Utilities|Array|AddUnique _targets _asbp_game_character)))))
  (return (LocalVariables|GetTargets)))

(fn RotatetoFaceTarget
  (params (Target :type Actor%20Object%20Reference))
  (Utilities|IsValid Target
    (:Is%20Valid
      (Transformation|SetWorldRotation (Variables|Collision|GetCapsuleComponent) (Math|Rotator|MakeRotator 0.0 0.0 (.yaw (Math|Rotator|FindLookatRotation (Transformation|GetActorLocation) (Transformation|GetActorLocation Target)))) false false))))

(fn CheckFinisherTargets
  (bind _capsulecomponent (Variables|Collision|GetCapsuleComponent))
  (bind _returnvalue (Transformation|GetWorldLocation _capsulecomponent))
  (bind (_outhits _returnvalue_2) (Class|KismetSystemLibrary|BoxTraceMulti _returnvalue (+ _returnvalue 1.0) "1500.000000,1500.000000,500.000000" "0, 0, 0" "TraceTypeQuery1" false 0 "None" true))
  (if _returnvalue_2
    (for _array_element _outhits
      (bind _asbp_monster_parent (Utilities|Casting|CastToBP_MonsterParent (.HitActor (Collision|BreakHitResult _array_element))))
      (if (Variables|BP_GameCharacter_C|GetisAlive _asbp_monster_parent)
        (if (< (Math|Conversions|ToFloat(Integer) (CallFunction|GetAttribute _asbp_monster_parent "NewEnumerator0")) (* (CallFunction|GetAttribute _asbp_monster_parent "NewEnumerator1") 0.2))
          (if (not (LocalVariables|Getdone))
            (LocalVariables|Setdone true)
            (CallFunction|Finisher1 _asbp_monster_parent)))))))
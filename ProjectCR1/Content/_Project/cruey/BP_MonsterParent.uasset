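; Base monster class handling player targeting, finisher prompts and finisher deaths.
; FindTarget box-traces for the closest pawn and targets the player only while fewer than two enemies are engaged; death decrements that count for minigame-room monsters.
; MonsterTick turns the finisher widget toward the player camera, showing it only on low-health flying bugs, and maintains a lock timer while finishers play.
; Receiving a finisher halts movement, then kills the monster after a delay.
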(event Custom|FindTarget
  (bind _value (CallFunction|GetAttribute "NewEnumerator4"))
  (bind _capsulecomponent (Variables|Default|GetCapsuleComponent))
  (bind _returnvalue (Transformation|GetWorldLocation _capsulecomponent))
  (bind _returnvalue_2 (Math|Conversions|ToFloat(Integer) _value))
  (bind _outhits (Class|KismetSystemLibrary|BoxTraceMultiforObjects _returnvalue (+ _returnvalue 1.0) (Math|Vector|MakeVector _returnvalue_2 _returnvalue_2 _returnvalue_2) "0, 0, 0" (Utilities|Array|MakeArray "ObjectTypeQuery3") false 0 "None" true))
  (Utilities|IsValid (CallFunction|GetClosestTarget (CallFunction|GetTargetsfromTraceHits _outhits))
    (:Is%20Valid
      (bind _asbp_player_character (Utilities|Casting|CastToBP_PlayerCharacter (CallFunction|GetClosestTarget (CallFunction|GetTargetsfromTraceHits _outhits))))
      (if (< (Variables|/Game/_Project/BP/Player/BP_PlayerCharacter.BP_PlayerCharacter_C|GetCurrentEnemiesEngaged_0 _asbp_player_character) 2)
        (bind _asbp_game_character (Utilities|Casting|CastToBP_GameCharacter (CallFunction|GetClosestTarget (CallFunction|GetTargetsfromTraceHits _outhits))))
        (bind _output_get (Variables|Default|SetTarget _asbp_game_character))
        (bind _asbp_player_character_2 (Utilities|Casting|CastToBP_PlayerCharacter _output_get))
        (bind _result (Math|Integer|IncrementInt (Variables|/Game/_Project/BP/Player/BP_PlayerCharacter.BP_PlayerCharacter_C|GetCurrentEnemiesEngaged_0 _asbp_player_character_2))
          (:%20%20
            (bind _output_get_2 (Variables|/Game/_Project/BP/Player/BP_PlayerCharacter.BP_PlayerCharacter_C|SetCurrentEnemiesEngaged_0 _asbp_player_character_2 _result))
            (Development|PrintString (Utilities|String|BuildString(Integer) "" "ENEMIES ENGAGED : " _output_get_2))))))))

(event Custom|DeleteFromMinigame
  (bind _self self)
  (bind _minigame_roomparent (Variables|Default|GetMinigame_RoomParent))
  (bind _asbp_player_character (CallFunction|GetPlayerChar _self))
  (Utilities|IsValid _minigame_roomparent
    (:Is%20Valid
      (Utilities|Array|RemoveItem (Variables|/Game/_Project/cruey/Minigame_System/BP_Room.BP_Room_C|GetMonsters _minigame_roomparent) self)
      (bind _result (Math|Integer|DecrementInt (Variables|/Game/_Project/BP/Player/BP_PlayerCharacter.BP_PlayerCharacter_C|GetCurrentEnemiesEngaged_0 _asbp_player_character))
        (:%20%20
          (bind _output_get (Variables|/Game/_Project/BP/Player/BP_PlayerCharacter.BP_PlayerCharacter_C|SetCurrentEnemiesEngaged_0 _asbp_player_character _result))
          (if (< _output_get 0)
            (Variables|/Game/_Project/BP/Player/BP_PlayerCharacter.BP_PlayerCharacter_C|SetCurrentEnemiesEngaged_0 _asbp_player_character 0))
          (Development|PrintString (Utilities|String|BuildString(Integer) "" "ENEMIES ENGAGED : " _output_get)))))))

(event EventBeginPlay)

(event Collision|EventActorBeginOverlap
  (params (OtherActor :type Actor%20Object%20Reference)))

(event EventBeginPlayMonster
  (EventDispatchers|BindEventtoOnDeath (delegate Custom|DeleteFromMinigame))
  (Utilities|FlowControl|Delay 3.0)
  (Actor|SetOwner (.AsBP%20Player%20Character (CallFunction|GetPlayerChar self))))

(event EventMonsterTick
  (bind _value (CallFunction|GetAttribute "NewEnumerator1"))
  (bind _value_2 (CallFunction|GetAttribute "NewEnumerator0"))
  (bind _self self)
  (bind _finisher_widget (Variables|Default|GetFINISHER_WIDGET))
  (bind _finisher_widget_2 (Variables|Default|GetFINISHER_WIDGET))
  (bind _returnvalue (Math|Conversions|ToFloat(Integer) _value))
  (bind _returnvalue_2 (Math|Conversions|ToFloat(Integer) _value_2))
  (bind _asbp_player_character (CallFunction|GetPlayerChar _self))
  (bind _returnvalue_3 (/ _returnvalue_2 _returnvalue))
  (if (not (Variables|Default|GetIsBeingAttacked))
    (Utilities|FlowControl|Sequence
      (:then_0
        (Utilities|IsValid _finisher_widget
          (:Is%20Valid
            (Utilities|IsValid _asbp_player_character
              (:Is%20Valid
                (Transformation|SetWorldRotation _finisher_widget (Math|Rotator|FindLookatRotation (Transformation|GetWorldLocation _finisher_widget) (Transformation|GetWorldLocation (Variables|/Game/_Project/BP/Player/BP_PlayerCharacter.BP_PlayerCharacter_C|GetCamera _asbp_player_character))) false false))))))
      (:then_1
        (Utilities|FlowControl|Sequence
          (:then_0
            (Utilities|IsValid (Variables|Default|GetW_Finish_Ref)
              (:Is%20Not%20Valid
                (bind _returnvalue_4 (UserInterface|CreateWidget "/Game/_Project/cruey/W_FINISH.W_FINISH_C"))
                (bind _output_get (Variables|Default|SetW_Finish_Ref _returnvalue_4))
                (UserInterface|SetWidget (Variables|Default|GetFINISHER_WIDGET) _output_get))))
          (:then_1
            (Utilities|Casting|CastToBP_FlyingBug self
              (:then
                (Rendering|SetVisibility _finisher_widget_2 (select (and (< _returnvalue_3 0.2) (> _returnvalue_3 0.01)) true false) false))
              (:CastFailed
                (Rendering|SetVisibility _finisher_widget_2 false false))))))
      (:then_2
        (if (> (Variables|Default|GetFullLock_Time) 0.0)
          (Variables|Default|SetFullLock_Time (- (Variables|Default|GetFullLock_Time) 1.0))))
      (:then_3
        (if (Variables|/Game/_Project/BP/Player/BP_PlayerCharacter.BP_PlayerCharacter_C|GetisUsingFinisher (.AsBP%20Player%20Character (CallFunction|GetPlayerChar self)))
          (Variables|Default|SetFullLock_Time 2.0))))))

(event EventRecieveFinisher
  (bind _charactermovement (Variables|Character|GetCharacterMovement))
  (Default|CallOnRecieveFinisher)
  (Variables|Default|SetFullLock_Time 2.0)
  (Variables|/Script/Engine.CharacterMovementComponent|SetMaxWalkSpeed _charactermovement 0.0)
  (Components|Movement|StopMovementImmediately _charactermovement)
  (Pawn|Components|CharacterMovement|SetMovementMode _charactermovement "MOVE_None" 0)
  (Utilities|FlowControl|Delay 2.0)
  (CallFunction|Die))

(fn ConstructionScript
  (|CallParentFunction))

(fn GetClosestTarget
  (params (Array :type Array%20of%20Actor%20Object%20References))
  (for _array_element Array
    (if (< (Math|Vector|Distance(Vector) (Transformation|GetActorLocation _array_element) (Transformation|GetWorldLocation (Variables|Default|GetCapsuleComponent))) (LocalVariables|GetDistance))
      (LocalVariables|SetDistance (Math|Vector|Distance(Vector) (Transformation|GetActorLocation _array_element) (Transformation|GetWorldLocation (Variables|Default|GetCapsuleComponent))))
      (LocalVariables|SetClosestTarget _array_element)))
  (return (LocalVariables|GetClosestTarget)))
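; BP_Projectile is a projectile actor that deals area damage when it meets something other than its owner.
; Sphere hit, character overlap and a per-tick overlap check all trigger Explode, guarded to run once.
; Explode damages overlapping BP_GameCharacters in the owner's TargetTypes through the owner's SendDamage, using an owner attribute as base damage.
; It destroys itself after a short delay.
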(event OnComponentHit(Sphere1)
  (params (HitComponent :type Primitive%20Component%20Object%20Reference) (OtherActor :type Actor%20Object%20Reference) (OtherComp :type Primitive%20Component%20Object%20Reference) (NormalImpulse :type Vector :default "0, 0, 0") (Hit :type Hit%20Result%20Structure%20%28by%20ref%29))
  (if (!= OtherActor (Components|GetOwner))
    (CallFunction|Explode)))

(event OnComponentBeginOverlap(Sphere1)
  (params (OverlappedComponent :type Primitive%20Component%20Object%20Reference) (OtherActor :type Actor%20Object%20Reference) (OtherComp :type Primitive%20Component%20Object%20Reference) (OtherBodyIndex :type Integer) (bFromSweep :type Boolean) (SweepResult :type Hit%20Result%20Structure%20%28by%20ref%29))
  (if (!= OtherActor (Components|GetOwner))
    (Utilities|Casting|CastToBP_GameCharacter OtherActor)
    (CallFunction|Explode)))

(event Custom|Explode
  (bind _returnvalue (Components|GetOwner))
  (bind _asbp_game_character (CallFunction|GetGameChar _returnvalue))
  (if (not (Variables|Default|GetExploded))
    (Variables|Default|SetExploded true)
    (for _array_element (Collision|GetOverlappingActors (Variables|Default|GetSphere1) "/Game/_Project/cruey/BP_GameCharacter.BP_GameCharacter_C" :!class /Script/Engine.PrimitiveComponent)
      (if (!= _array_element _asbp_game_character)
        (bind _asbp_game_character_2 (Utilities|Casting|CastToBP_GameCharacter _array_element))
        (if (Utilities|Array|ContainsItem (Variables|/Game/_Project/cruey/BP_GameCharacter.BP_GameCharacter_C|GetTargetTypes _asbp_game_character) (Variables|/Game/_Project/cruey/BP_GameCharacter.BP_GameCharacter_C|GetTargetGroup _asbp_game_character_2))
          (Default|SendDamage _asbp_game_character _array_element (Math|Conversions|ToFloat(Integer) (Default|GetAttribute _asbp_game_character "NewEnumerator2")) 0 false))))
    (Utilities|FlowControl|Delay 5.0)
    (Actor|DestroyActor)))

(event EventBeginPlay)

(event Collision|EventActorBeginOverlap
  (params (OtherActor :type Actor%20Object%20Reference)))

(event EventTick
  (params (DeltaSeconds :type Float%20%28single-precision%29))
  (if (not (Variables|Default|GetExploded))
    (for _array_element (Collision|GetOverlappingActors (Variables|Default|GetSphere1) "/Game/_Project/cruey/BP_GameCharacter.BP_GameCharacter_C" :!class /Script/Engine.PrimitiveComponent)
      (if (!= _array_element (Components|GetOwner))
        (CallFunction|Explode)))))

(fn ConstructionScript)
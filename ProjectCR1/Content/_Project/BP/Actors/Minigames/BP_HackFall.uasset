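; BP_HackFall is a dodge-the-falling-hazards hacking minigame with three lives and a survival countdown.
; Setup blurs the view through MPC_Blur, spawns and possesses a BP_HackPlayer, and switches to a spawned camera.
; A looping timer drops random hazard patterns while a timeline slides the player between two side markers.
; Win or game over fades out, restores BP_PlayerCharacter and removes spawned player and camera; only winning activates ActorToActivate.
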(event Custom|Setup
  (bind _camerapos (Variables|Default|GetCameraPos))
  (bind _rightside (Variables|Default|GetRightSide))
  (Variables|Default|Setlives 3)
  (bind _returnvalue (Game|SpawnActorfromClass "/Game/_Project/BP/Player/BP_HackPlayer.BP_HackPlayer_C" (Math|Transform|MakeTransform (Transformation|GetWorldLocation _rightside) (Transformation|GetWorldRotation _rightside) "1,1,1") "Undefined" 0 self 0))
  (Variables|Default|SetPlayer _returnvalue)
  (bind _returnvalue_2 (Game|SpawnActorfromClass "/Game/_Project/BP/Actors/Camera/BP_Camera.BP_Camera_C" (Math|Transform|MakeTransform (Transformation|GetWorldLocation _camerapos) (Transformation|GetWorldRotation _camerapos) "1,1,1") "Undefined" 0 0))
  (Variables|Default|SetCamera _returnvalue_2)
  (CallFunction|DoBlur)
  (Utilities|FlowControl|Delay 1.4)
  (Game|Player|SetViewTargetwithBlend (Game|GetPlayerController 0) _returnvalue_2 0.0 "VTBlend_Linear" 0.0 false)
  (CameraFades|StartCameraFade (Game|GetPlayerCameraManager 0) 1.0 0.0 1.0 "(R=1.000000,G=1.000000,B=1.000000,A=1.000000)" false true)
  (Utilities|FlowControl|Delay 1.2)
  (Pawn|Possess (Game|GetPlayerController 0) (Variables|Default|GetPlayer))
  (Game|Player|SetViewTargetwithBlend (Game|GetPlayerController 0) (Variables|Default|GetCamera) 0.0 "VTBlend_Linear" 0.0 false)
  (CallFunction|StartPlay))

(event Custom|MoveToLeft
  (Variables|Default|GetPlayer
    (:then
      (Variables|Default|Setmovingleft true)
      (bind _alpha (Timeline|MovePlayer Play)
        (:Update
          (Transformation|SetActorLocation (Variables|Default|GetPlayer) (Math|Vector|Lerp(Vector) (Transformation|GetWorldLocation (Variables|Default|GetRightSide)) (Transformation|GetWorldLocation (Variables|Default|GetLeftSide)) _alpha) false false))))
    (:else)))

(event Custom|Countdown
  (bind _output_get (Variables|Default|SetcurrentTimer (- (Variables|Default|GetcurrentTimer) 1)))
  (if (<= _output_get 0)
    (Utilities|Time|ClearandInvalidateTimerbyHandle (stale Custom|init_TimerTimer _returnvalue))
    (CallFunction|WinState)))

(event Custom|WinState
  (Variables|Default|SetinPlay false)
  (Collision|SetCollisionEnabled (Variables|/Game/_Project/BP/Player/BP_HackPlayer.BP_HackPlayer_C|GetPlayer (Variables|Default|GetPlayer)) "NoCollision")
  (CameraFades|StartCameraFade (Game|GetPlayerCameraManager 0) 0.0 1.0 1.0 "(R=1.000000,G=1.000000,B=1.000000,A=1.000000)" false true)
  (Utilities|FlowControl|Delay 2.0)
  (bind _returnvalue (Actor|GetActorOfClass "/Game/_Project/BP/Player/BP_PlayerCharacter.BP_PlayerCharacter_C"))
  (Game|Player|SetViewTargetwithBlend (Game|GetPlayerController 0) _returnvalue 0.0 "VTBlend_Linear" 0.0 false)
  (CallFunction|UnBlur)
  (Utilities|FlowControl|Delay 0.2)
  (Actor|DestroyActor (Variables|Default|GetPlayer))
  (Variables|Default|SetPlayer 0)
  (Actor|DestroyActor (Variables|Default|GetCamera))
  (Variables|Default|SetCamera 0)
  (Pawn|Possess (Game|GetPlayerController 0) _returnvalue)
  (CameraFades|StartCameraFade (Game|GetPlayerCameraManager 0) 1.0 0.0 1.0 "(R=1.000000,G=1.000000,B=1.000000,A=1.000000)" false true)
  (Utilities|FlowControl|Delay 2.0)
  (Variables|/Game/_Project/BP/Player/BP_PlayerCharacter.BP_PlayerCharacter_C|SetEPS _returnvalue "NewEnumerator0")
  (Class|BPIWorldEvents|DoActivate(Message) (Variables|Default|GetActorToActivate)))

(event Custom|DoBlur
  (bind _bluritup (Timeline|BlurFX PlayFromStart)
    (:Update
      (Rendering|Material|SetScalarParameterValue "/Game/_Project/Art/PP/MPC_Blur.MPC_Blur" "BlurDist" _bluritup :!class /Script/Engine.KismetMaterialLibrary))
    (:Finished
      (Rendering|Material|SetScalarParameterValue "/Game/_Project/Art/PP/MPC_Blur.MPC_Blur" "BlurDist" 0.0 :!class /Script/Engine.KismetMaterialLibrary))))

(event Custom|UnBlur
  (bind _bluritup (Timeline|BlurFX ReverseFromEnd)
    (:Update
      (Rendering|Material|SetScalarParameterValue "/Game/_Project/Art/PP/MPC_Blur.MPC_Blur" "BlurDist" _bluritup :!class /Script/Engine.KismetMaterialLibrary))
    (:Finished
      (Rendering|Material|SetScalarParameterValue "/Game/_Project/Art/PP/MPC_Blur.MPC_Blur" "BlurDist" 0.0 :!class /Script/Engine.KismetMaterialLibrary))))

(event Custom|MoveToRight
  (Variables|Default|GetPlayer
    (:then
      (Variables|Default|Setmovingleft false)
      (bind _alpha (Timeline|MovePlayer Reverse)
        (:Update
          (Transformation|SetActorLocation (Variables|Default|GetPlayer) (Math|Vector|Lerp(Vector) (Transformation|GetWorldLocation (Variables|Default|GetRightSide)) (Transformation|GetWorldLocation (Variables|Default|GetLeftSide)) _alpha) false false))))
    (:else)))

(event Custom|StartPlay
  (Variables|Default|SetinPlay true)
  (CallFunction|InitSpawnHazardTimer)
  (Variables|Default|SetcurrentTimer (Variables|Default|GetTimeToPass))
  (CallFunction|InitTimerTimer))

(event Custom|LoseLife
  (bind _output_get (Variables|Default|Setlives (- (Variables|Default|Getlives) 1)))
  (if (<= _output_get 0)
    (CallFunction|GameOver)
    (bind _alpha (Timeline|MovePlayer Stop)
      (:Update
        (Transformation|SetActorLocation (Variables|Default|GetPlayer) (Math|Vector|Lerp(Vector) (Transformation|GetWorldLocation (Variables|Default|GetRightSide)) (Transformation|GetWorldLocation (Variables|Default|GetLeftSide)) _alpha) false false)))))

(event Custom|GameOver
  (Variables|Default|SetinPlay false)
  (Utilities|Time|ClearandInvalidateTimerbyHandle (Variables|Default|GetTimer))
  (Collision|SetCollisionEnabled (Variables|/Game/_Project/BP/Player/BP_HackPlayer.BP_HackPlayer_C|GetPlayer (Variables|Default|GetPlayer)) "NoCollision")
  (CameraFades|StartCameraFade :self (Game|GetPlayerCameraManager 0) :ToAlpha 1.0 :Duration 1.0 :bHoldWhenFinished true)
  (Utilities|FlowControl|Delay 2.0)
  (bind _returnvalue (Actor|GetActorOfClass "/Game/_Project/BP/Player/BP_PlayerCharacter.BP_PlayerCharacter_C"))
  (Game|Player|SetViewTargetwithBlend (Game|GetPlayerController 0) _returnvalue 0.0 "VTBlend_Linear" 0.0 false)
  (CallFunction|UnBlur)
  (Utilities|FlowControl|Delay 0.2)
  (Actor|DestroyActor (Variables|Default|GetPlayer))
  (Variables|Default|SetPlayer 0)
  (Actor|DestroyActor (Variables|Default|GetCamera))
  (Variables|Default|SetCamera 0)
  (Pawn|Possess (Game|GetPlayerController 0) _returnvalue)
  (CameraFades|StartCameraFade :self (Game|GetPlayerCameraManager 0) :FromAlpha 1.0 :Duration 1.0 :bHoldWhenFinished true)
  (Utilities|FlowControl|Delay 2.0)
  (Variables|/Game/_Project/BP/Player/BP_PlayerCharacter.BP_PlayerCharacter_C|SetEPS _returnvalue "NewEnumerator0"))

(event Custom|InitSpawnHazardTimer
  (Utilities|Time|SetTimerbyEvent (delegate Custom|CheckifCanSpawnHazard) 0.5 true))

(event Custom|CheckifCanSpawnHazard
  (if (Variables|Default|GetinPlay)
    (switch int (Math|Random|RandomIntegerinRange 0 8)
      (:1
        (CallFunction|SpawnHazard 0.0))
      (:2
        (CallFunction|SpawnHazard -2e+02))
      (:3
        (CallFunction|SpawnHazard -1.5e+02))
      (:4
        (CallFunction|SpawnHazard 1.5e+02))
      (:5
        (CallFunction|SpawnHazard 2e+02))
      (:6
        (CallFunction|SpawnHazard -2e+02)
        (CallFunction|SpawnHazard 2e+02))
      (:7
        (CallFunction|SpawnHazard 1e+02)
        (CallFunction|SpawnHazard 2e+02))
      (:8
        (CallFunction|SpawnHazard -1e+02)
        (CallFunction|SpawnHazard -2e+02)))))

(event Custom|SpawnHazard
  (params (Ypos :type Float%20%28single-precision%29))
  (Game|SpawnActorfromClass "/Game/_Project/BP/Actors/Minigames/BP_HF_Hazard1.BP_HF_Hazard1_C" (Math|Transform|MakeTransform (+ (Transformation|GetWorldLocation (Variables|Default|GetFallFrom)) (Math|Vector|MakeVector 0.0 Ypos 0.0)) "0, 0, 0" "1,1,1") "Undefined" 0 self 0))

(event Custom|init_TimerTimer
  (bind _returnvalue (Utilities|Time|SetTimerbyEvent (delegate Custom|Countdown) 1.0 true))
  (Variables|Default|SetTimer _returnvalue))

(fn ConstructionScript)
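; BP_ITest is a test interactable actor that gives visible feedback by randomizing the colour of its Cube.
; TryInteract sets the Colour vector parameter on the cube's materials to random RGB values, then clears the interacting player's CurrentInteractable.
; DoActivate applies the same random recolour without touching any player state.
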(event EventDoActivate
  (Rendering|Material|SetVectorParameterValueonMaterials (Variables|Default|GetCube) "Colour" (Math|Vector|MakeVector (Math|Random|RandomFloatinRange 0.0 1.0) (Math|Random|RandomFloatinRange 0.0 1.0) (Math|Random|RandomFloatinRange 0.0 1.0))))

(event EventTryInteract
  (params (Player :type BP%20Player%20Character%20Object%20Reference))
  (Rendering|Material|SetVectorParameterValueonMaterials (Variables|Default|GetCube) "Colour" (Math|Vector|MakeVector (Math|Random|RandomFloatinRange 0.0 1.0) (Math|Random|RandomFloatinRange 0.0 1.0) (Math|Random|RandomFloatinRange 0.0 1.0)))
  (Variables|/Game/_Project/BP/Player/BP_PlayerCharacter.BP_PlayerCharacter_C|SetcurrentInteractable Player 0))

(fn ConstructionScript)
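; BP_Dummy is a damageable dummy enemy that respawns in place after being killed.
; While alive, incoming damage plays a timeline that animates the cube's Colour material parameter and is passed as a negative change to the ACHealth component.
; When the health update returns true, it hides the cube and its children, waits briefly, restores full health, and unhides only the cube before becoming alive again.
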(event Custom|TakeDamageFX
  (bind _colour (Timeline|DamageColourFX PlayFromStart)
    (:Update
      (Rendering|Material|SetVectorParameterValueonMaterials (Variables|Default|GetCube) "Colour" _colour))))

(event Custom|Death
  (bind _ac_health (Variables|Default|GetAC_Health))
  (Development|SetHiddeninGame (Variables|Default|GetCube) true true)
  (Utilities|FlowControl|Delay 2.0)
  (Variables|/Game/_Project/BP/Comps/AC_Health.AC_Health_C|SetcurrentHealth _ac_health (Variables|/Game/_Project/BP/Comps/AC_Health.AC_Health_C|GetMAX_HEALTH _ac_health))
  (Development|SetHiddeninGame (Variables|Default|GetCube) false false)
  (Variables|Default|Setalive? true))

(event Game|Damage|EventAnyDamage
  (params (Damage :type Float%20%28single-precision%29) (DamageType :type Damage%20Type%20Object%20Reference) (InstigatedBy :type Controller%20Object%20Reference) (DamageCauser :type Actor%20Object%20Reference))
  (if (Variables|Default|Getalive?)
    (CallFunction|TakeDamageFX)
    (bind _dead_ (Default|UpdateHealth (Variables|Default|GetAC_Health) (* Damage -1.0)))
    (if _dead_
      (Variables|Default|Setalive? false)
      (CallFunction|Death))))

(fn ConstructionScript)
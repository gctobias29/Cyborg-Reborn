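; Player character Blueprint with camera-yaw-relative movement, cooldown-limited dash, combo attacks and interaction, gated mostly by the EPS state.
; Light, heavy and elemental attacks track combo counters by last attack type, with heavy or elemental after light resetting the count.
; Attacks face the aim stick or mouse cursor, then use placeholder prints and a damaging debug box trace instead of animations.
; Interaction line-traces forward for BPI_Interact actors and relays try, continue and release messages.
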(event Input|ActionEvents|InputActionInteract
  (params (Key :type Key%20Structure :default "None"))
  ;[1 1 1] Interaction System
  (:Pressed
    (if (Variables|Status|GetcanAction?)
      (switch Utilities|FlowControl|Switch|SwitchonEPlayerState (Variables|Status|GetEPS)
        (:NewEnumerator0
          (bind _found_ (CallFunction|LookforInteraction))
          (if _found_
            _))
        (:NewEnumerator1
          (bind _currentinteractable (Variables|Refs|GetcurrentInteractable)
            (:then
              (Class|BPIInteract|ContinueInteract(Message) _currentinteractable self))
            (:else
              (Variables|Status|SetEPS "NewEnumerator0")))))))
  (:Released
    (switch Utilities|FlowControl|Switch|SwitchonEPlayerState (Variables|Status|GetEPS)
      (:NewEnumerator1
        (bind _currentinteractable_2 (Variables|Refs|GetcurrentInteractable)
          (:then
            (Class|BPIInteract|ReleaseInteract(Message) _currentinteractable_2 self))
          (:else))))))

(event Input|ActionEvents|InputActionLightAtk
  (params (Key :type Key%20Structure :default "None"))
  ;[1 1 1] Attack System Initial
  (:Pressed
    (switch Utilities|FlowControl|Switch|SwitchonEPlayerState (Variables|Status|GetEPS)
      (:NewEnumerator0
        (if (Variables|Status|GetcanAction?)
          (Variables|Status|SetcanAction? false)
          (if (Utilities|Enum|Equal(Enum) (Variables|Combat|GetLastAttack) "NewEnumerator0")
            _
            (else
              (Variables|Combat|SetcomboCounter 0)))
          ;;[1 1 1] Do Attack - Can Action Var should set back to true at end of animation via Anim Notify
          (CallFunction|FaceAttackRot)
          (Development|PrintString (Utilities|String|BuildString(Integer) "" "Light Attack : " (Variables|Combat|GetcomboCounter)))
          (CallFunction|DebugAttack)
          (Variables|Status|SetcanAction? true)
          (CallFunction|AddtoComboCounter (Variables|Combat|GetMaxLightAttackCombo))
          (Variables|Combat|SetLastAttack "NewEnumerator0"))))))

(event Input|ActionEvents|InputActionHeavyAtk
  (params (Key :type Key%20Structure :default "None"))
  ;[1 1 1] Attack System Initial
  (:Pressed
    (switch Utilities|FlowControl|Switch|SwitchonEPlayerState (Variables|Status|GetEPS)
      (:NewEnumerator0
        (if (Variables|Status|GetcanAction?)
          (Variables|Status|SetcanAction? false)
          (if (Utilities|Enum|Equal(Enum) (Variables|Combat|GetLastAttack) "NewEnumerator0")
            (CallFunction|FaceAttackRot)
            (Development|PrintString (Utilities|String|BuildString(Integer) "" "Heavy Attack : " (Variables|Combat|GetcomboCounter)))
            (CallFunction|DebugAttack)
            (Variables|Status|SetcanAction? true)
            (Variables|Combat|SetcomboCounter 0)
            (else
              ;;[1 1 1] Do Attack - Can Action Var should set back to true at end of animation via Anim Notify
              (CallFunction|FaceAttackRot)
              (Development|PrintString (Utilities|String|BuildString(Integer) "" "Heavy Attack : " (Variables|Combat|GetcomboCounter)))
              (CallFunction|DebugAttack)
              (Variables|Status|SetcanAction? true)
              (CallFunction|AddtoComboCounter (Variables|Combat|GetMaxHeavyCombo))))
          (Variables|Combat|SetLastAttack "NewEnumerator1"))))))

(event Input|ActionEvents|InputActionElemAtk
  (params (Key :type Key%20Structure :default "None"))
  ;[1 1 1] Attack System Initial
  (:Pressed
    (switch Utilities|FlowControl|Switch|SwitchonEPlayerState (Variables|Status|GetEPS)
      (:NewEnumerator0
        (if (Variables|Status|GetcanAction?)
          (Variables|Status|SetcanAction? false)
          (if (Utilities|Enum|Equal(Enum) (Variables|Combat|GetLastAttack) "NewEnumerator0")
            (CallFunction|FaceAttackRot)
            (Development|PrintString (Utilities|String|BuildString(Integer) "" "Elemental Attack : " (Variables|Combat|GetcomboCounter)))
            (CallFunction|DebugAttack)
            (Variables|Status|SetcanAction? true)
            (Variables|Combat|SetcomboCounter 0)
            (else
              ;;[1 1 1] Do Attack - Can Action Var should set back to true at end of animation via Anim Notify
              (CallFunction|FaceAttackRot)
              (Development|PrintString (Utilities|String|BuildString(Integer) "" "Elemental Attack : " (Variables|Combat|GetcomboCounter)))
              (CallFunction|DebugAttack)
              (Variables|Status|SetcanAction? true)
              (CallFunction|AddtoComboCounter (Variables|Combat|GetMaxElementalCombo))))
          (Variables|Combat|SetLastAttack "NewEnumerator2"))))))

(event Input|ActionEvents|InputActionDash
  (params (Key :type Key%20Structure :default "None"))
  ;[1 1 1] Dash
  (:Pressed
    (if (and (Utilities|Enum|Equal(Enum) (Variables|Status|GetEPS) "NewEnumerator0") (Variables|Status|GetcanDash?))
      (Variables|Status|SetcanDash? false)
      (Variables|Status|SetcanAction? false)
      (Character|LaunchCharacter (* (Math|Vector|Normalize (Pawn|Components|CharacterMovement|GetCurrentAcceleration (Variables|Character|GetCharacterMovement))) (Variables|Stats|GetDashAmount)) true true)
      (Utilities|FlowControl|RetriggerableDelay 0.15)
      (Variables|Status|SetcanAction? true)
      (Utilities|FlowControl|RetriggerableDelay 0.85)
      (Variables|Status|SetcanDash? true))))

(event Input|AxisEvents|InputAxisMoveForward
  (params (AxisValue :type Float%20%28single-precision%29))
  ;[1 1 1] Movement
  (if (Utilities|Enum|Equal(Enum) (Variables|Status|GetEPS) "NewEnumerator0")
    (Pawn|Input|AddMovementInput (Math|Vector|GetForwardVector (Math|Rotator|MakeRotator 0.0 0.0 (.yaw (Transformation|GetWorldRotation (Variables|Default|GetCamera))))) AxisValue false)))

(event Input|AxisEvents|InputAxisMoveRight
  (params (AxisValue :type Float%20%28single-precision%29))
  ;[1 1 1] Movement
  (if (Utilities|Enum|Equal(Enum) (Variables|Status|GetEPS) "NewEnumerator0")
    (Pawn|Input|AddMovementInput (Math|Vector|GetRightVector (Math|Rotator|MakeRotator 0.0 0.0 (.yaw (Transformation|GetWorldRotation (Variables|Default|GetCamera))))) AxisValue false)))

(fn ConstructionScript)

(fn FaceAttackRot
  (bind _returnvalue (Game|GetPlayerController 0))
  (bind (_hitresult _returnvalue_2) (Game|Player|GetHitResultUnderCursorbyChannel _returnvalue "TraceTypeQuery3" true))
  (if (or (> (Math|Float|Absolute(Float) (Input|AxisValues|GetC_AimRight)) 0.0) (> (Math|Float|Absolute(Float) (Input|AxisValues|GetC_AimUp)) 0.0))
    (Transformation|SetActorRotation (Math|Rotator|MakeRotator 0.0 0.0 (+ (.yaw (Math|Rotator|MakeRotfromX (Math|Vector|MakeVector (* (Input|AxisValues|GetC_AimUp) -1.0) (Input|AxisValues|GetC_AimRight) 0.0))) -45.0)))
    (elif (not (Variables|Controls|GetusingController))
      (if _returnvalue_2
        (Transformation|SetActorRotation (Math|Rotator|MakeRotator 0.0 0.0 (.Yaw (Math|Rotator|BreakRotator (Math|Rotator|FindLookatRotation (Transformation|GetActorLocation) (.ImpactPoint (Collision|BreakHitResult _hitresult)))))))))))

(fn LookforInteraction
  (bind _returnvalue (Transformation|GetActorLocation))
  (bind (_outhit _returnvalue_2) (Collision|LineTraceByChannel _returnvalue (+ _returnvalue (* (Transformation|GetActorForwardVector) 1e+02)) "TraceTypeQuery1" false 0 "None"))
  (if _returnvalue_2
    (if (Utilities|DoesObjectImplementInterface (.HitActor (Collision|BreakHitResult _outhit)) "/Game/_Project/BP/Static/BPI/BPI_Interact.BPI_Interact_C")
      (bind _output_get (Variables|Refs|SetcurrentInteractable (.HitActor (Collision|BreakHitResult _outhit))))
      (Class|BPIInteract|TryInteract(Message) _output_get self)
      (return true)
      (else
        _)))
  (return false))

(fn AddtoComboCounter
  (params (MaxCombo :type Integer))
  (if (>= (Variables|Combat|GetcomboCounter) MaxCombo)
    (Variables|Combat|SetcomboCounter 0)
    (else
      (Variables|Combat|SetcomboCounter (+ (Variables|Combat|GetcomboCounter) 1)))))

(fn DebugAttack
  (bind _returnvalue (Transformation|GetActorLocation))
  (bind (_outhits _returnvalue_2) (Class|KismetSystemLibrary|BoxTraceMulti _returnvalue (+ _returnvalue (* (Transformation|GetActorForwardVector) 1.5e+02)) "0,90.000000,50.000000" (Transformation|GetActorRotation) "TraceTypeQuery1" false 0 "ForOneFrame" true))
  (if _returnvalue_2
    (for _array_element _outhits
      (Game|Damage|ApplyDamage (.HitActor (Collision|BreakHitResult _array_element)) 1.0 0 0))))
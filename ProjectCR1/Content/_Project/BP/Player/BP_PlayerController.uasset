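; BP_PlayerController is the player controller that creates the HUD, moves the character's cursor to the mouse world location each tick and toggles pause on Escape or P.
; Left click triggers a move on a possessed BP_HackPlayer; otherwise it box-traces for pawns at the cursor to choose an attack.
; A living BP_FlyingBug at or below a 20% attribute ratio (likely health) receives a finisher, while healthier monsters or empty clicks trigger a light attack.
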(event Custom|TogglePause
  (bind _output_get (Variables|Default|SetPaused (select (Variables|Default|GetPaused) false true)))
  (Game|SetGamePaused _output_get))

(event EventBeginPlay
  (bind _returnvalue (UserInterface|CreateWidget "/Game/_Project/cruey/W_HUD.W_HUD_C"))
  (Variables|Default|Sethudref _returnvalue)
  (UserInterface|Viewport|AddtoViewport _returnvalue 0))

(event EventTick
  (params (DeltaSeconds :type Float%20%28single-precision%29))
  (Transformation|SetWorldLocation (Variables|/Game/_Project/BP/Player/BP_PlayerCharacter.BP_PlayerCharacter_C|Getcursor (.AsBP%20Player%20Character (CallFunction|GetPlayerChar self))) (.Location (CallFunction|MouseWorldLoc self)) false false))

(event Input|MouseEvents|LeftMouseButton
  (params (Key :type Key%20Structure :default "None"))
  (bind _self self)
  (bind _self_2 self)
  (bind _asbp_player_character (CallFunction|GetPlayerChar _self))
  (bind _location (CallFunction|MouseWorldLoc _self_2))
  (:Pressed
    (bind _asbp_hack_player (Utilities|Casting|CastToBP_HackPlayer (Pawn|GetControlledPawn))
      (:then
        (Default|TriggerMove _asbp_hack_player))
      (:CastFailed
        (bind _outhit (Class|KismetSystemLibrary|BoxTraceSingleforObjects _location _location "100.000000,100.000000,200.000000" "0, 0, 0" (Utilities|Array|MakeArray "ObjectTypeQuery3") false 0 "None" true))
        (if (.bBlockingHit (Collision|BreakHitResult _outhit))
          (bind _asbp_monster_parent (Utilities|Casting|CastToBP_MonsterParent (.HitActor (Collision|BreakHitResult _outhit))))
          (if (> (/ (Math|Conversions|ToFloat(Integer) (Default|GetAttribute _asbp_monster_parent "NewEnumerator0")) (Math|Conversions|ToFloat(Integer) (Default|GetAttribute _asbp_monster_parent "NewEnumerator1"))) 0.2)
            (Default|TriggerLIghtAttack _asbp_player_character :!label _label)
            (elif (Variables|/Game/_Project/cruey/BP_GameCharacter.BP_GameCharacter_C|GetisAlive _asbp_monster_parent)
              (bind _asbp_flying_bug (Utilities|Casting|CastToBP_FlyingBug _asbp_monster_parent))
              (Development|PrintString "trigger finish")
              (Default|Finisher1 _asbp_player_character _asbp_flying_bug)
              (else
                (goto _label))))
          (else
            (Default|TriggerLIghtAttack _asbp_player_character)))))))

(event Input|KeyboardEvents|P
  (params (Key :type Key%20Structure :default "None"))
  (:Pressed
    (CallFunction|TogglePause)))

(event Input|KeyboardEvents|Escape
  (params (Key :type Key%20Structure :default "None"))
  (:Pressed
    (CallFunction|TogglePause)))

(fn ConstructionScript)
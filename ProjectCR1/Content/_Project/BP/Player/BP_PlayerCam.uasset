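; Player camera actor that smoothly follows the player character and keeps it in view.
; Each tick, the Camera interpolates toward a point blended between its current location and the character's DefaultCam, while easing its rotation to look at the character.
; It also switches SpringArm collision testing on in cinematic mode and off otherwise.
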(event EventBeginPlay)

(event Collision|EventActorBeginOverlap
  (params (OtherActor :type Actor%20Object%20Reference)))

(event EventTick
  (params (DeltaSeconds :type Float%20%28single-precision%29))
  (bind _self self)
  (bind _springarm (Variables|Default|GetSpringArm))
  (bind _camera (Variables|Default|GetCamera))
  (bind _asbp_player_character (CallFunction|GetPlayerChar _self))
  (bind _returnvalue (Transformation|GetWorldLocation _camera))
  (Variables|Default|SetDelta%20Seconds DeltaSeconds)
  (Utilities|FlowControl|Sequence
    (:then_0
      (Transformation|SetWorldLocationAndRotation _camera (Math|Interpolation|VInterpTo _returnvalue (Math|Vector|Lerp(Vector) _returnvalue (Transformation|GetWorldLocation (Variables|/Game/_Project/BP/Player/BP_PlayerCharacter.BP_PlayerCharacter_C|GetDefaultCam _asbp_player_character)) 0.6) (Variables|Default|GetDelta%20Seconds) 2.0) (Math|Interpolation|RInterpTo (Transformation|GetWorldRotation (Variables|Default|GetCamera)) (Math|Rotator|FindLookatRotation (Transformation|GetWorldLocation (Variables|Default|GetCamera)) (Transformation|GetActorLocation _asbp_player_character)) (Variables|Default|GetDelta%20Seconds) 2.0) false true))
    (:then_1
      (if (CallFunction|GetCinematicMode self)
        (Variables|/Script/Engine.SpringArmComponent|SetbDoCollisionTest _springarm true)
        (else
          (Variables|/Script/Engine.SpringArmComponent|SetbDoCollisionTest _springarm false))))))

(fn ConstructionScript)